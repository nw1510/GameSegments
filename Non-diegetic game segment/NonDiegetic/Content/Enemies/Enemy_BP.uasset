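; Enemy pawn that roams to random reachable points until it spots the player, then chases and attacks.
; PawnSensing sets CanSeePlayer, which is never cleared, and starts an AIMoveTo chase that opens a timed attack window on arrival, then repeats.
; A Sphere overlap during that window damages the ThirdPersonCharacter once per attack and plays a warning sound when the player's health is low.
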(event `self.ReceiveBeginPlay`
  (`|AIMoveTo` self (`NavigationSystemV1.K2_GetRandomReachablePointInRadius` (`self.K2_GetActorLocation`) 10000.0 null null) null :!label _label
    (:`OnSuccess`
      (if (not (`self.CanSeePlayer`))
        (goto _label)))))

(event `self.PawnSensing.OnSeePawn`
  (params (Pawn :type "Pawn Object Reference"))
  (bind _asthird_person_character (cast `/Game/ThirdPersonBP/Blueprints/ThirdPersonCharacter` Pawn))
  (set `self.CanSeePlayer` true)
  (`|AIMoveTo` self (0.0 0.0 0.0) _asthird_person_character :!label _label_2
    (:`OnSuccess`
      (if (not (`self.Attacking`))
        (set `self.Attacking` true)
        (`KismetSystemLibrary.Delay` 2.3)
        (set `self.Attacking` false)
        (set `self.AlreadyHit` false)
        (goto _label_2)))))

(event `self.Sphere.OnComponentBeginOverlap`
  (params (OverlappedComponent :type "PrimitiveComponent Object Reference") (OtherActor :type "Actor Object Reference") (OtherComp :type "PrimitiveComponent Object Reference") (OtherBodyIndex :type Integer) (bFromSweep :type Boolean) (SweepResult :type "HitResult Structure (by ref)"))
  (bind _asthird_person_character (cast `/Game/ThirdPersonBP/Blueprints/ThirdPersonCharacter` OtherActor))
  (if (`self.Attacking`)
    (if (not (`self.AlreadyHit`))
      (bind _output_get (set `/Game/ThirdPersonBP/Blueprints/ThirdPersonCharacter.CurrentHealth` (- (`/Game/ThirdPersonBP/Blueprints/ThirdPersonCharacter.CurrentHealth` _asthird_person_character) 100.0) _asthird_person_character))
      (set `self.AlreadyHit` true)
      (if (<= _output_get 100.0)
        (`GameplayStatics.PlaySound2D` "/Game/Enemies/Warning_Cue.Warning_Cue" 1.0 1.0 0.0 null null)))))

(fn `UserConstructionScript`)