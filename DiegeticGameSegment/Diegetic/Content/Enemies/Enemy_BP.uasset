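; Enemy pawn that roams randomly until it spots the player, then chases and attacks.
; AI MoveTo loops drive wandering, re-rolled when enemies bump, until PawnSensing permanently sets CanSeePlayer and switches to pursuit.
; Reaching the player opens a timed attack window in which sphere overlap deals one hit, activating player damage components and a warning sound at low health thresholds.
; It also links its health bar widget and clears the lightning ability's Chained flag.
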(event `self.Box.OnComponentBeginOverlap`
  (params (OverlappedComponent :type "PrimitiveComponent Object Reference") (OtherActor :type "Actor Object Reference") (OtherComp :type "PrimitiveComponent Object Reference") (OtherBodyIndex :type Integer) (bFromSweep :type Boolean) (SweepResult :type "HitResult Structure (by ref)"))
  ;[1 1 1] If enemies bump into eachother when they cant see the player, move to another spot within a 10000 radius. Prevents enemies from getting stuck on eachother
  (cast `/Game/Enemies/Enemy_BP` OtherActor)
  (if (not (`self.CanSeePlayer`))
    ;[1 1 1] If enemy can't see the player. Continue to move to a random point within a 10,000 radius
    (`|AIMoveTo` self (`NavigationSystemV1.K2_GetRandomReachablePointInRadius` (`self.K2_GetActorLocation`) 10000.0 null null) null :!label _label
      (:`OnSuccess`
        (if (not (`self.CanSeePlayer`))
          (goto _label))))))

(event `self.ReceiveBeginPlay`
  ;[1 1 1] On begin play, set the enemy health bar to belong to that enemy
  (bind _asenemy_health_ui (cast `/Game/UI/EnemyHealthUI` (`WidgetComponent.GetUserWidgetObject` (`self.HealthBar`))))
  (set `/Game/UI/EnemyHealthUI.OwningEnemy` self _asenemy_health_ui)
  (goto _label))

(event `self.PawnSensing.OnSeePawn`
  (params (Pawn :type "Pawn Object Reference"))
  ;[1 1 1] When the enemy sees the player, mover to the player and begin attacking then continue to move to player character
  (bind _asthird_person_character (cast `/Game/ThirdPersonBP/Blueprints/ThirdPersonCharacter` Pawn))
  (set `self.CanSeePlayer` true)
  (`|AIMoveTo` self (0.0 0.0 0.0) _asthird_person_character :!label _label_2
    (:`OnSuccess`
      (if (not (`self.Attacking`))
        (set `self.Attacking` true)
        (`KismetSystemLibrary.Delay` 2.3)
        (set `self.Attacking` false)
        (set `self.AlreadyHit` false)
        (goto _label_2)))))

(event `self.Sphere.OnComponentBeginOverlap`
  (params (OverlappedComponent :type "PrimitiveComponent Object Reference") (OtherActor :type "Actor Object Reference") (OtherComp :type "PrimitiveComponent Object Reference") (OtherBodyIndex :type Integer) (bFromSweep :type Boolean) (SweepResult :type "HitResult Structure (by ref)"))
  ;[1 1 1] When the sphere collision overlaps with the player character, take away 100 health from the player. Play a warning sound when the player is below 100 health.
  (bind _asthird_person_character (cast `/Game/ThirdPersonBP/Blueprints/ThirdPersonCharacter` OtherActor))
  (if (`self.Attacking`)
    (if (not (`self.AlreadyHit`))
      (bind _output_get (set `/Game/ThirdPersonBP/Blueprints/ThirdPersonCharacter.CurrentHealth` (- (`/Game/ThirdPersonBP/Blueprints/ThirdPersonCharacter.CurrentHealth` _asthird_person_character) 100.0) _asthird_person_character))
      (set `self.AlreadyHit` true)
      (if (<= _output_get 500.0)
        (`ActorComponent.Activate` (`/Game/ThirdPersonBP/Blueprints/ThirdPersonCharacter.DamageLeftShoulder` _asthird_person_character) false)
        (`ActorComponent.Activate` (`/Game/ThirdPersonBP/Blueprints/ThirdPersonCharacter.DamageLeftLeg` _asthird_person_character) false)
        (if (<= _output_get 250.0)
          (`ActorComponent.Activate` (`/Game/ThirdPersonBP/Blueprints/ThirdPersonCharacter.DamageRightShoulder` _asthird_person_character) false)
          (`ActorComponent.Activate` (`/Game/ThirdPersonBP/Blueprints/ThirdPersonCharacter.DamageRightLeg` _asthird_person_character) false)
          (`GameplayStatics.PlaySound2D` "/Game/Enemies/DamageZap_Cue.DamageZap_Cue" 1.0 1.0 0.0 null null))))))

(event `self.ReceiveTick`
  (params (DeltaSeconds :type "Float (single-precision)"))
  ;[1 1 1] Sets chained variable back to false after 0.1 seconds. Used for the lightning ability.
  (if (`self.Chained`)
    (`KismetSystemLibrary.Delay` 0.1)
    (set `self.Chained` false)))

(fn `UserConstructionScript`)